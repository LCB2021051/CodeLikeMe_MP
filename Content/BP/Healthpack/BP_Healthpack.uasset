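; BP_Healthpack is a health pickup with an animated billboard, collected when an actor overlaps its box.
; A Timeline restarts after a short pause and scales the billboard's screen size, toggling visibility twice per update, likely to refresh it.
; Overlap sends CollectHealthMessage to the other actor through a DoOnce gate.
; A true result expires the pack via a short lifespan; otherwise the gate resets.
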(event `self.ReceiveBeginPlay`
  (bind _billboard (`self.Billboard`))
  (bind (_direction _time) (`Timeline|Timeline` :!label _label)
    (:`Update`
      (set `BillboardComponent.ScreenSize` (* _time 0.003) _billboard)
      (`SceneComponent.ToggleVisibility` _billboard false)
      (`SceneComponent.ToggleVisibility` _billboard false))
    (:`Finished`
      (`KismetSystemLibrary.Delay` 0.2)
      (goto _label :!via `PlayFromStart`))))

(event `self.Box.OnComponentBeginOverlap`
  (params (OverlappedComponent :type "PrimitiveComponent Object Reference") (OtherActor :type "Actor Object Reference") (OtherComp :type "PrimitiveComponent Object Reference") (OtherBodyIndex :type Integer) (bFromSweep :type Boolean) (SweepResult :type "HitResult Structure (by ref)"))
  (`/Engine/EditorBlueprintResources/StandardMacros.DoOnce` false :!label _label_2
    (:`Completed`
      (bind _collected (message `/Game/FirstPerson/Blueprints/BPI_MP_Character.CollectHealth` OtherActor 1.0))
      (if _collected
        (`self.SetLifeSpan` 0.1)
        (else
          (goto _label_2 :!via `Reset`))))))

(fn `UserConstructionScript`)